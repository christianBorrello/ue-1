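; BP_SlashCharacter is a character Blueprint that configures hair for an Echo-based character in its construction script.
; A UseGroomAssets flag picks groom hair and eyebrows with their bindings, without physics, or a skeletal hair mesh driven by its own AnimBP for physics.
; The event graph holds only empty placeholder events, so the Blueprint adds no runtime logic.
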(event EventBeginPlay)

(event Collision|EventActorBeginOverlap
  (params (OtherActor :type Actor%20Object%20Reference)))

(event EventTick
  (params (DeltaSeconds :type Float%20%28single-precision%29)))

(fn ConstructionScript
  (if (Variables|Default|GetUseGroomAssets)
    ;[1 1 1] Hair Groom without physics
    (Class|GroomComponent|SetGroomAsset (Variables|Default|GetHairGroom) "/Game/Static/EchoContent/Characters/Echo/Hair/Hair_S_UpdoBuns.Hair_S_UpdoBuns")
    (Class|GroomComponent|SetBindingAsset (Variables|Default|GetHairGroom) "/Game/Static/EchoContent/Characters/Echo/Hair/Hair_S_UpdoBuns_Echo_M3D_LOD0_Binding.Hair_S_UpdoBuns_Echo_M3D_LOD0_Binding")
    (Class|GroomComponent|SetGroomAsset (Variables|Default|GetEyebrowsGroom) "/Game/Static/EchoContent/Characters/Echo/Hair/Eyebrows_L_Echo.Eyebrows_L_Echo")
    (Class|GroomComponent|SetBindingAsset (Variables|Default|GetEyebrowsGroom) "/Game/Static/EchoContent/Characters/Echo/Hair/Eyebrows_L_Echo_Echo_M3D_LOD0_Binding.Eyebrows_L_Echo_Echo_M3D_LOD0_Binding")
    (else
      ;[1 1 1] Skeletal Mesh Hair with Physics Bodies
      (Components|SkinnedMesh|SetSkinnedAssetandUpdate (Variables|Default|GetHairMesh) "/Game/Static/EchoContent/Characters/Echo/Meshes/Echo_Hair.Echo_Hair" true)
      (Class|SkeletalMeshComponent|SetAnimClass (Variables|Default|GetHairMesh) "/Game/Static/EchoContent/Characters/Echo/Rig/Echo_Hair_AnimBP.Echo_Hair_AnimBP_C"))))